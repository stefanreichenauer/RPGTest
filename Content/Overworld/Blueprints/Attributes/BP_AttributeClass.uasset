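; Attribute class for the overworld that tracks level and experience for seven character attributes, from Strength and Defense to Speed and Health.
; AddAttributeExp selects the attribute's struct by enum and adds experience, or on reaching the threshold increments the level and carries over the surplus, one level per call.
; GetNextLevelExpFromDataTable then writes the new threshold by reference from the AttributeLevel table row named after the new level.
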(fn AddAttributeExp
  (params (Attribute :type E_Attributes%20Enum :default "NewEnumerator0") (ExpValue :type Integer))
  (bind _attributes (Variables|Default|GetAttributes))
  (bind (_strength _defense _intelligence _faith _dexterity _speed _health) (Utilities|Struct|BreakS_Attributes _attributes))
  (bind _returnvalue (Utilities|Select :Index Attribute :NewEnumerator0 _strength :NewEnumerator1 _defense :NewEnumerator2 _intelligence :NewEnumerator3 _faith :NewEnumerator4 _dexterity :NewEnumerator5 _speed :NewEnumerator6 _health))
  (bind (_level _actualexp _nextlevelexp) (Utilities|Struct|BreakS_AttributeExp _returnvalue))
  (bind _returnvalue_2 (+ ExpValue _actualexp))
  (if (>= _returnvalue_2 _nextlevelexp)
    (bind _result (Math|Integer|IncrementInt _level)
      (:%20%20
        (Utilities|Struct|SetmembersinS_AttributeExp _returnvalue (- _returnvalue_2 _nextlevelexp))
        (Utilities|GetNextLevelExpfromDataTable _result _nextlevelexp Attribute)))
    (else
      (Utilities|Struct|SetmembersinS_AttributeExp _returnvalue _returnvalue_2))))