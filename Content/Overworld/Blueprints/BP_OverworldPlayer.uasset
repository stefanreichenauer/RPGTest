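; BP_OverworldPlayer is the player-controlled pawn for the overworld, with axis-driven movement and look.
; MoveForward and MoveRight move along the actor's forward and right vectors, while the look axes drive controller yaw and inverted pitch.
; On BeginPlay, if no Inventory is valid, it spawns a BP_Inventory actor, adds two "Trank" items by name and prints each item's name and map value as debug output.
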(event EventBeginPlay
  (Utilities|IsValid (Variables|Default|GetInventory)
    (:Is%20Not%20Valid
      (bind _returnvalue (Game|SpawnActorfromClass "/Game/Overworld/Blueprints/BP_Inventory.BP_Inventory_C" (Transformation|GetActorTransform) "Undefined" 0 0))
      (bind _output_get (Variables|Default|SetInventory _returnvalue))
      (Default|AddItembyName _output_get "Trank")
      (Default|AddItembyName _output_get "Trank")
      (bind _keys (Utilities|Map|Keys (Variables|/Game/Overworld/Blueprints/BP_Inventory.BP_Inventory_C|GetItemList _output_get)))
      (for _array_element _keys
        (Development|PrintString (Utilities|String|ToString(Text) (Variables|/Game/Overworld/Blueprints/BP_Item.BP_Item_C|GetName _array_element)))
        (Development|PrintString (Utilities|String|ToString(Integer) (.Value (Utilities|Map|Find (Variables|/Game/Overworld/Blueprints/BP_Inventory.BP_Inventory_C|GetItemList _output_get) _array_element))))))))

(event Collision|EventActorBeginOverlap
  (params (OtherActor :type Actor%20Object%20Reference)))

(event EventTick
  (params (DeltaSeconds :type Float%20%28single-precision%29)))

(event Input|AxisEvents|InputAxisMoveForward
  (params (AxisValue :type Float%20%28single-precision%29))
  (Pawn|Input|AddMovementInput (Transformation|GetActorForwardVector) AxisValue false))

(event Input|AxisEvents|InputAxisMoveRight
  (params (AxisValue :type Float%20%28single-precision%29))
  (Pawn|Input|AddMovementInput (Transformation|GetActorRightVector) AxisValue false))

(event Input|AxisEvents|InputAxisLookHorizontal
  (params (AxisValue :type Float%20%28single-precision%29))
  (Pawn|Input|AddControllerYawInput AxisValue))

(event Input|AxisEvents|InputAxisLookVertical
  (params (AxisValue :type Float%20%28single-precision%29))
  (Pawn|Input|AddControllerPitchInput (* AxisValue -1.0)))

(fn ConstructionScript)