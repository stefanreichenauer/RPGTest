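; Base actor Blueprint for usable overworld items, providing a UseItem function that consumes the item from the player's inventory.
; UseItem prints the item's Name, casts the first player pawn to BP_OverworldPlayer and asks it to remove that Name from the inventory.
; It applies no item effect of its own, and the event graph holds only disabled placeholder events.
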(event EventBeginPlay
  (|CallParentFunction) ; This node is disabled and will not be called.\nDrag off pins to build functionality.
)

(event Collision|EventActorBeginOverlap
  (params (OtherActor :type Actor%20Object%20Reference))
  (|CallParentFunction OtherActor) ; This node is disabled and will not be called.\nDrag off pins to build functionality.
)

(event EventTick
  (params (DeltaSeconds :type Float%20%28single-precision%29))
  (|CallParentFunction DeltaSeconds) ; This node is disabled and will not be called.\nDrag off pins to build functionality.
)

(fn ConstructionScript
  (|CallParentFunction))

(fn UseItem
  (Development|PrintString (Utilities|String|Append "Used Item: " (Utilities|String|ToString(Text) (Variables|Default|GetName))))
  (bind _asbp_overworld_player (Utilities|Casting|CastToBP_OverworldPlayer (Game|Player|GetPlayerPawn 0)))
  (Default|RemoveItemfromInventory _asbp_overworld_player (Variables|Default|GetName)))