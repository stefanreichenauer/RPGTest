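; BP_WeaponSword is an equippable sword weapon for the overworld, built on a parent class that supplies its setup.
; Its Attack function caches the wielder's and target's attributes, then switches on attack type, but no case is wired yet.
; Two unconnected damage formulas weight Strength and Dexterity differently, multiply by Damage and subtract the target's Defense.
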(event EventBeginPlay
  (|CallParentFunction))

(event Collision|EventActorBeginOverlap
  (params (OtherActor :type Actor%20Object%20Reference))
  (|CallParentFunction OtherActor) ; This node is disabled and will not be called.\nDrag off pins to build functionality.
)

(event EventTick
  (params (DeltaSeconds :type Float%20%28single-precision%29))
  (|CallParentFunction DeltaSeconds) ; This node is disabled and will not be called.\nDrag off pins to build functionality.
)

(fn ConstructionScript
  (|CallParentFunction))

(fn Attack
  (params (AttackType :type Byte :default 0) (Target :type I%20Character%20Interface))
  (bind _attributes (Default|GetAttributes (Variables|Default|GetWielder)))
  (LocalVariables|SetAttackerAttributes _attributes)
  (bind _attributes_2 (Default|GetAttributes Target))
  (LocalVariables|SetTargetAttributes _attributes_2)
  (switch Utilities|FlowControl|Switch|Switchon AttackType))