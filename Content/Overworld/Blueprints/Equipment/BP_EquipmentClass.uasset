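; Equipment manager that tracks worn armor and two weapons in an equipment struct and maintains a running total defense.
; EquipItem first unequips any item in the target slot, then stores the cast armor or weapon, adding armor defense to the total.
; Unequipping returns the item to the linked inventory by name, subtracts that slot's defense and clears it; weapon slots contribute no defense.
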(fn EquipItem
  (params (Item :type BP%20Equippable%20Item%20Object%20Reference) (Slot :type E_EquipmentSlots%20Enum :default "NewEnumerator0"))
  (bind _equipment (Variables|Default|GetEquipment))
  (bind (_headgear _chestgear _leggear _footgear _handgear _primaryweapon _secondaryweapon) (Utilities|Struct|BreakS_EquipmentObjects _equipment))
  (switch Utilities|FlowControl|Switch|SwitchonE_EquipmentSlots Slot
    (:NewEnumerator0
      (Utilities|UnequipItemifSet _headgear Slot
        (:Out
          (bind _asbp_armor_item (Utilities|Casting|CastToBP_ArmorItem Item))
          (Utilities|Struct|SetmembersinS_EquipmentObjects (Variables|Default|GetEquipment) _asbp_armor_item)
          (bind _asbp_armor_item_2 (Utilities|Casting|CastToBP_ArmorItem Item :!label _label))
          (Variables|Default|SetEquipmentDefense (+ (Variables|Default|GetEquipmentDefense) (Variables|/Game/Overworld/Blueprints/Items/Armor/BP_ArmorItem.BP_ArmorItem_C|GetDefence _asbp_armor_item_2))))))
    (:NewEnumerator1
      (Utilities|UnequipItemifSet _chestgear Slot
        (:Out
          (bind _asbp_armor_item_3 (Utilities|Casting|CastToBP_ArmorItem Item))
          (Utilities|Struct|SetmembersinS_EquipmentObjects (Variables|Default|GetEquipment) _asbp_armor_item_3)
          (goto _label))))
    (:NewEnumerator2
      (Utilities|UnequipItemifSet _leggear Slot
        (:Out
          (bind _asbp_armor_item_4 (Utilities|Casting|CastToBP_ArmorItem Item))
          (Utilities|Struct|SetmembersinS_EquipmentObjects (Variables|Default|GetEquipment) _asbp_armor_item_4)
          (goto _label))))
    (:NewEnumerator3
      (Utilities|UnequipItemifSet _footgear Slot
        (:Out
          (bind _asbp_armor_item_5 (Utilities|Casting|CastToBP_ArmorItem Item))
          (Utilities|Struct|SetmembersinS_EquipmentObjects (Variables|Default|GetEquipment) _asbp_armor_item_5)
          (goto _label))))
    (:NewEnumerator4
      (Utilities|UnequipItemifSet _handgear Slot
        (:Out
          (bind _asbp_armor_item_6 (Utilities|Casting|CastToBP_ArmorItem Item))
          (Utilities|Struct|SetmembersinS_EquipmentObjects (Variables|Default|GetEquipment) _asbp_armor_item_6)
          (goto _label))))
    (:NewEnumerator5
      (Utilities|UnequipItemifSet _primaryweapon Slot
        (:Out
          (bind _asbp_weapon_item (Utilities|Casting|CastToBP_WeaponItem Item))
          (Utilities|Struct|SetmembersinS_EquipmentObjects (Variables|Default|GetEquipment) _asbp_weapon_item))))
    (:NewEnumerator6
      (Utilities|UnequipItemifSet _secondaryweapon Slot
        (:Out
          (bind _asbp_weapon_item_2 (Utilities|Casting|CastToBP_WeaponItem Item))
          (Utilities|Struct|SetmembersinS_EquipmentObjects (Variables|Default|GetEquipment) _asbp_weapon_item_2))))))

(fn UnequipItem
  (params (Item :type BP%20Equippable%20Item%20Object%20Reference) (Slot :type E_EquipmentSlots%20Enum :default "NewEnumerator0"))
  (Default|AddItemtoInventory (Variables|Default|GetInventory) (Utilities|Struct|BreakItemObjectAttributes (Variables|/Game/Overworld/Blueprints/Items/BP_BaseItemObject.BP_BaseItemObject_C|GetItemAttributes Item)))
  (CallFunction|ResetEquipmentSlot Slot))

(fn ResetEquipmentSlot
  (params (Slot :type E_EquipmentSlots%20Enum :default "NewEnumerator0"))
  (bind _defense (CallFunction|GetDefenseOfSlot Slot))
  (Variables|Default|SetEquipmentDefense (- (Variables|Default|GetEquipmentDefense) _defense))
  (switch Utilities|FlowControl|Switch|SwitchonE_EquipmentSlots Slot
    (:NewEnumerator0
      (Utilities|Struct|SetmembersinS_EquipmentObjects (Variables|Default|GetEquipment)))
    (:NewEnumerator1
      (Utilities|Struct|SetmembersinS_EquipmentObjects (Variables|Default|GetEquipment)))
    (:NewEnumerator2
      (Utilities|Struct|SetmembersinS_EquipmentObjects (Variables|Default|GetEquipment)))
    (:NewEnumerator3
      (Utilities|Struct|SetmembersinS_EquipmentObjects (Variables|Default|GetEquipment)))
    (:NewEnumerator4
      (Utilities|Struct|SetmembersinS_EquipmentObjects (Variables|Default|GetEquipment)))
    (:NewEnumerator5
      (Utilities|Struct|SetmembersinS_EquipmentObjects (Variables|Default|GetEquipment)))
    (:NewEnumerator6
      (Utilities|Struct|SetmembersinS_EquipmentObjects (Variables|Default|GetEquipment)))))

(fn GetDefenseOfSlot
  (params (Slot :type E_EquipmentSlots%20Enum :default "NewEnumerator0"))
  (bind _equipment (Variables|Default|GetEquipment))
  (bind (_headgear _chestgear _leggear _footgear _handgear) (Utilities|Struct|BreakS_EquipmentObjects _equipment))
  (switch Utilities|FlowControl|Switch|SwitchonE_EquipmentSlots Slot
    (:NewEnumerator0
      (LocalVariables|SetArmor _headgear))
    (:NewEnumerator1
      (LocalVariables|SetArmor _chestgear))
    (:NewEnumerator2
      (LocalVariables|SetArmor _leggear))
    (:NewEnumerator3
      (LocalVariables|SetArmor _footgear))
    (:NewEnumerator4
      (LocalVariables|SetArmor _handgear))
    (:NewEnumerator5
      (return 0))
    (:NewEnumerator6
      (return 0)))
  (Utilities|IsValid (LocalVariables|GetArmor)
    (:Is%20Valid
      (return (Variables|/Game/Overworld/Blueprints/Items/Armor/BP_ArmorItem.BP_ArmorItem_C|GetDefence (LocalVariables|GetArmor))))
    (:Is%20Not%20Valid
      (return 0))))

(fn SetInventoryReference
  (params (NewParam :type BP%20Inventory%20Class%20Object%20Reference%20%28by%20ref%29))
  (Variables|Default|SetInventory NewParam))