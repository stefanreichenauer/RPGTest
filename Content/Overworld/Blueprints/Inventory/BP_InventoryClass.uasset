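; BP_InventoryClass is the overworld inventory, storing items as item-and-count structs in ItemList.
; Adding increments an existing stack or constructs a new item object.
; The enum-keyed path looks up ItemObjectTable for class and attributes, while the older-style name path creates a bare BP_BaseItemObject.
; Removal exists only by name and re-appends decremented stacks at the list's end.
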(fn GetItembyName
  (params (ItemName :type Text))
  (for (_array_element _array_index) (Variables|Default|GetItemList)
    (if (Utilities|Enum|Equal(Enum) (Variables|/Game/Overworld/Blueprints/Items/BP_BaseItemObject.BP_BaseItemObject_C|GetName (.Item (Utilities|Struct|BreakS_Inventory _array_element))) ItemName)
      (return (.Item (Utilities|Struct|BreakS_Inventory _array_element)) _array_index))))

(fn AddItemtoInventorybyName
  (params (ItemName :type Text))
  (bind (_item _arrayindex) (CallFunction|GetItembyName ItemName))
  (Utilities|IsValid _item
    (:Is%20Valid
      (Utilities|Array|SetArrayElem (Variables|Default|GetItemList) _arrayindex (Utilities|Struct|MakeS_Inventory (.Item (Utilities|Struct|BreakS_Inventory (Utilities|Array|Get(acopy) (Variables|Default|GetItemList) _arrayindex))) (+ (.Count (Utilities|Struct|BreakS_Inventory (Utilities|Array|Get(acopy) (Variables|Default|GetItemList) _arrayindex))) 1))))
    (:Is%20Not%20Valid
      (bind _returnvalue (Game|ConstructObjectfromClass "/Game/Overworld/Blueprints/Items/BP_BaseItemObject.BP_BaseItemObject_C" self))
      (Variables|/Game/Overworld/Blueprints/Items/BP_BaseItemObject.BP_BaseItemObject_C|SetName _returnvalue ItemName)
      (Utilities|Array|Add (Variables|Default|GetItemList) (Utilities|Struct|MakeS_Inventory _returnvalue 1)))))

(fn RemoveItemfromInventorybyName
  (params (ItemName :type Text))
  (bind _itemlist (Variables|Default|GetItemList))
  (bind (_item _arrayindex) (CallFunction|GetItembyName ItemName))
  (Utilities|IsValid _item
    (:Is%20Valid
      (if (> (- (.Count (Utilities|Struct|BreakS_Inventory (Utilities|Array|Get(acopy) (Variables|Default|GetItemList) _arrayindex))) 1) 0)
        (Utilities|Array|Add _itemlist (Utilities|Struct|MakeS_Inventory (.Item (Utilities|Struct|BreakS_Inventory (Utilities|Array|Get(acopy) (Variables|Default|GetItemList) _arrayindex))) (- (.Count (Utilities|Struct|BreakS_Inventory (Utilities|Array|Get(acopy) (Variables|Default|GetItemList) _arrayindex))) 1))))
      (Utilities|Array|RemoveIndex _itemlist _arrayindex))))

(fn GetItem
  (params (ItemName :type E_UsableItemList%20Enum :default "NewEnumerator0"))
  (for (_array_element _array_index) (Variables|Default|GetItemList)
    (if (Utilities|Enum|Equal(Enum) (.Name (Utilities|Struct|BreakItemObjectAttributes (Variables|/Game/Overworld/Blueprints/Items/BP_BaseItemObject.BP_BaseItemObject_C|GetItemAttributes (Utilities|Struct|BreakS_Inventory _array_element)))) ItemName)
      (Development|PrintString 0 (Utilities|String|Append "Fond ITem: " (Utilities|String|EnumtoString (.Name (Utilities|Struct|BreakItemObjectAttributes (Variables|/Game/Overworld/Blueprints/Items/BP_BaseItemObject.BP_BaseItemObject_C|GetItemAttributes (Utilities|Struct|BreakS_Inventory _array_element)))))))
      (return (Utilities|Struct|BreakS_Inventory _array_element) _array_index))))

(fn AddItemtoInventory
  (params (Item :type E_UsableItemList%20Enum :default "NewEnumerator0"))
  (bind (_item _arrayindex) (CallFunction|GetItem Item))
  (Utilities|IsValid _item
    (:Is%20Valid
      (Utilities|Array|SetArrayElem (Variables|Default|GetItemList) _arrayindex (Utilities|Struct|MakeS_Inventory (.Item (Utilities|Struct|BreakS_Inventory (Utilities|Array|Get(acopy) (Variables|Default|GetItemList) _arrayindex))) (+ (.Count (Utilities|Struct|BreakS_Inventory (Utilities|Array|Get(acopy) (Variables|Default|GetItemList) _arrayindex))) 1))))
    (:Is%20Not%20Valid
      (bind _item_2 (CallFunction|FindIteminDataTable Item))
      (bind _returnvalue (Game|ConstructObjectfromClass (.ItemType (Utilities|Struct|BreakItemObjectAttributes _item_2)) self))
      (Variables|/Game/Overworld/Blueprints/Items/BP_BaseItemObject.BP_BaseItemObject_C|SetItemAttributes _returnvalue _item_2)
      (Utilities|Array|Add (Variables|Default|GetItemList) (Utilities|Struct|MakeS_Inventory _returnvalue 1)))))

(fn FindIteminDataTable
  (params (Name :type E_UsableItemList%20Enum :default "NewEnumerator0"))
  (bind _outrownames (DataTable|GetDataTableRowNames "/Game/Overworld/Blueprints/Items/ItemObjectTable.ItemObjectTable"))
  (for _array_element _outrownames
    (bind _returnvalue (Utilities|GetDataTableRow "/Game/Overworld/Blueprints/Items/ItemObjectTable.ItemObjectTable" _array_element)
      (:then
        (if (Utilities|Enum|Equal(Enum) (Utilities|Struct|BreakItemObjectAttributes _returnvalue) Name)
          (return _returnvalue))))))