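; Overworld player character handling movement, camera look, a toggleable menu, inventory, equipment slots and attribute leveling.
; On begin play it seeds test items, puts a sword into the game instance equipment, registers itself there and moves to the stored overworld transform.
; Inventory stacks items by name, and attribute experience levels up using thresholds from a data table.
; Debug keys test language switching, experience gain, armor creation and saving or loading the transform.
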(event Custom|CloseInventory
  (bind _returnvalue (Game|GetPlayerController 0))
  (bind _returnvalue_2 (Game|GetPlayerController 0))
  ;[1 1 1] Inventory
  (if (not (Variables|Default|GetInUI))
    (Utilities|IsValid (Variables|Default|GetMenuWidget)
      (:Is%20Not%20Valid
        (bind _returnvalue_3 (UserInterface|CreateWidget "/Game/Overworld/Widgets/WT_Menu.WT_Menu_C"))
        (Widget|SetKeyboardFocus _returnvalue_3)
        (bind _output_get (Variables|Default|SetMenuWidget _returnvalue_3))
        (Default|SetMenuPlayer _output_get self)
        (Default|ConstructMenuWidget _returnvalue_3)
        (UserInterface|Viewport|AddtoViewport _returnvalue_3 0)
        (Input|SetInputModeGameandUI _returnvalue_2 _returnvalue_3 "DoNotLock" true)
        (Variables|/Script/Engine.PlayerController|SetbShowMouseCursor _returnvalue_2 true)
        (Variables|Default|SetInUI true)))
    (else
      (Utilities|IsValid (Variables|Default|GetMenuWidget)
        (:Is%20Valid
          (Widget|RemovefromParent (Variables|Default|GetMenuWidget))
          (Input|SetInputModeGameOnly _returnvalue)
          (Variables|/Script/Engine.PlayerController|SetbShowMouseCursor _returnvalue false)
          (Variables|Default|SetInUI false)
          (Variables|Default|SetMenuWidget 0))))))

(event EventBeginPlay
  (bind _returnvalue (Game|GetGameInstance))
  (Input|SetInputModeGameOnly (Game|GetPlayerController 0))
  (Inventory|AddItemtoInventory "Test1")
  (Inventory|AddItemtoInventory "Test2")
  (Inventory|AddItemtoInventory "Test1")
  (bind _returnvalue_2 (Game|SpawnActorfromClass "/Game/Overworld/Blueprints/Items/ItemActors/BP_BaseItemUsable.BP_BaseItemUsable_C" (Transformation|GetActorTransform) "Undefined" 0 0))
  (Variables|/Game/Overworld/Blueprints/Items/ItemActors/BP_BaseItem.BP_BaseItem_C|SetName _returnvalue_2 "Potion")
  (Utilities|Array|Add (Variables|Default|GetInventoryList) (Utilities|Struct|MakeBP_Inventory _returnvalue_2 1))
  (bind _returnvalue_3 (Game|ConstructObjectfromClass "/Game/Overworld/Blueprints/Items/Weapons/BP_SwordItem.BP_SwordItem_C" _returnvalue))
  (Default|ConstructSwordItem _returnvalue_3)
  (bind _asbp_my_game_instance (Utilities|Casting|CastToBP_MyGameInstance _returnvalue))
  (Utilities|Struct|SetmembersinS_EquipmentObjects (Variables|/Game/Overworld/Blueprints/Equipment/BP_EquipmentClass.BP_EquipmentClass_C|GetEquipment (Variables|/Game/GameInstance/BP_PlayerCharacteristics.BP_PlayerCharacteristics_C|GetEquipment (Variables|/Game/GameInstance/BP_MyGameInstance.BP_MyGameInstance_C|GetPlayerCharacteristics _asbp_my_game_instance))) _returnvalue_3)
  (Variables|/Game/GameInstance/BP_MyGameInstance.BP_MyGameInstance_C|SetOverworldPlayer _asbp_my_game_instance self)
  (Transformation|SetActorTransform (Variables|/Game/GameInstance/BP_MyGameInstance.BP_MyGameInstance_C|GetOverworldTransform _asbp_my_game_instance) false true))

(event Collision|EventActorBeginOverlap
  (params (OtherActor :type Actor%20Object%20Reference)))

(event EventTick
  (params (DeltaSeconds :type Float%20%28single-precision%29)))

(event Input|ActionEvents|InputActionToggleInventory
  (params (Key :type Key%20Structure))
  (bind _returnvalue (Game|GetPlayerController 0))
  (bind _returnvalue_2 (Game|GetPlayerController 0))
  ;[1 1 1] Inventory
  (:Pressed
    (if (not (Variables|Default|GetInUI))
      (Utilities|IsValid (Variables|Default|GetMenuWidget)
        (:Is%20Not%20Valid
          (bind _returnvalue_3 (UserInterface|CreateWidget "/Game/Overworld/Widgets/WT_Menu.WT_Menu_C"))
          (Widget|SetKeyboardFocus _returnvalue_3)
          (bind _output_get (Variables|Default|SetMenuWidget _returnvalue_3))
          (Default|SetMenuPlayer _output_get self)
          (Default|ConstructMenuWidget _returnvalue_3)
          (UserInterface|Viewport|AddtoViewport _returnvalue_3 0)
          (Input|SetInputModeGameandUI _returnvalue_2 _returnvalue_3 "DoNotLock" true)
          (Variables|/Script/Engine.PlayerController|SetbShowMouseCursor _returnvalue_2 true)
          (Variables|Default|SetInUI true)))
      (else
        (Utilities|IsValid (Variables|Default|GetMenuWidget)
          (:Is%20Valid
            (Widget|RemovefromParent (Variables|Default|GetMenuWidget))
            (Input|SetInputModeGameOnly _returnvalue)
            (Variables|/Script/Engine.PlayerController|SetbShowMouseCursor _returnvalue false)
            (Variables|Default|SetInUI false)
            (Variables|Default|SetMenuWidget 0)))))))

(event Input|AxisEvents|InputAxisMoveForward
  (params (AxisValue :type Float%20%28single-precision%29))
  ;[1 1 1] Movement
  (if (not (Variables|Default|GetInUI))
    (Pawn|Input|AddMovementInput (Transformation|GetActorForwardVector) AxisValue false)
    (if (!= AxisValue 0.0)
      (Variables|Default|SetIsMovingForward true)
      (else
        (Variables|Default|SetIsMovingForward false)))))

(event Input|AxisEvents|InputAxisMoveRight
  (params (AxisValue :type Float%20%28single-precision%29))
  ;[1 1 1] Movement
  (if (not (Variables|Default|GetInUI))
    (Pawn|Input|AddMovementInput (Transformation|GetActorRightVector) AxisValue false)
    (if (!= AxisValue 0.0)
      (Variables|Default|SetIsMovingRight true)
      (else
        (Variables|Default|SetIsMovingRight false)))))

(event Input|AxisEvents|InputAxisLookHorizontal
  (params (AxisValue :type Float%20%28single-precision%29))
  ;[1 1 1] Movement
  (if (not (Variables|Default|GetInUI))
    (Pawn|Input|AddControllerYawInput AxisValue)))

(event Input|AxisEvents|InputAxisLookVertical
  (params (AxisValue :type Float%20%28single-precision%29))
  ;[1 1 1] Movement
  (if (not (Variables|Default|GetInUI))
    (Pawn|Input|AddControllerPitchInput (* AxisValue -1.0))))

(event Input|KeyboardEvents|V
  (params (Key :type Key%20Structure))
  (bind _attributes (Variables|Default|GetAttributes))
  (bind _strength (Utilities|Struct|BreakS_Attributes _attributes))
  (bind _actualexp (Utilities|Struct|BreakS_AttributeExp _strength))
  (bind _returnvalue (Utilities|String|ToString(Integer) _actualexp))
  (:Pressed
    (Development|PrintString (Utilities|String|Append "Exp: " _returnvalue))
    (Attributes|AddExptoAttribute 10 "Strength")
    (Development|PrintString (Utilities|String|Append "New Exp: " _returnvalue))))

(event Input|KeyboardEvents|M
  (params (Key :type Key%20Structure))
  ;[1 1 1] Save and Load Game
  (:Pressed
    (bind _returnvalue (SaveGame|CreateSaveGameObject "/Game/GameInstance/BP_MySaveGame.BP_MySaveGame_C"))
    (Variables|Default|SetMySaveGame _returnvalue)
    (bind _returnvalue_2 (SaveGame|LoadGamefromSlot (Variables|/Game/GameInstance/BP_MySaveGame.BP_MySaveGame_C|GetSaveSlotName _returnvalue) (Variables|/Game/GameInstance/BP_MySaveGame.BP_MySaveGame_C|GetUserIndex _returnvalue)))
    (bind _asbp_my_save_game (Utilities|Casting|CastToBP_MySaveGame _returnvalue_2))
    (Transformation|SetActorTransform (Variables|/Game/GameInstance/BP_MySaveGame.BP_MySaveGame_C|GetOverworldTransform _asbp_my_save_game) false true)
    (Pawn|SetControlRotation (Pawn|GetController) (.Rotation (Math|Transform|BreakTransform (Variables|/Game/GameInstance/BP_MySaveGame.BP_MySaveGame_C|GetOverworldTransform _asbp_my_save_game))))
    (Development|PrintString "Loaded  Game")))

(event Input|KeyboardEvents|K
  (params (Key :type Key%20Structure))
  (:Pressed
    (Class|KismetInternationalizationLibrary|SetCurrentLanguageandLocale "de")))

(event Input|KeyboardEvents|O
  (params (Key :type Key%20Structure))
  (bind _returnvalue (Game|GetGameInstance))
  (:Pressed
    (Development|PrintString "Set Inventory")
    (bind _asbp_my_game_instance (Utilities|Casting|CastToBP_MyGameInstance _returnvalue)
      (:then
        (bind _returnvalue_2 (Game|ConstructObjectfromClass "/Game/Overworld/Blueprints/Items/Armor/BP_ArmorItem.BP_ArmorItem_C" _returnvalue))
        (Variables|/Game/Overworld/Blueprints/Items/Armor/BP_ArmorItem.BP_ArmorItem_C|SetDefence _returnvalue_2 20))
      (:CastFailed
        (Development|PrintString "Cast failed")))))

(event Input|KeyboardEvents|N
  (params (Key :type Key%20Structure))
  ;[1 1 1] Save and Load Game
  (:Pressed
    (bind _returnvalue (SaveGame|CreateSaveGameObject "/Game/GameInstance/BP_MySaveGame.BP_MySaveGame_C"))
    (bind _output_get (Variables|Default|SetMySaveGame _returnvalue))
    (Variables|/Game/GameInstance/BP_MySaveGame.BP_MySaveGame_C|SetOverworldTransform _output_get (Transformation|GetActorTransform))
    (SaveGame|SaveGametoSlot _returnvalue (Variables|/Game/GameInstance/BP_MySaveGame.BP_MySaveGame_C|GetSaveSlotName _returnvalue) (Variables|/Game/GameInstance/BP_MySaveGame.BP_MySaveGame_C|GetUserIndex _returnvalue))
    (Development|PrintString "Saved Game")))

(fn ConstructionScript)

(fn GetItembyName
  (params (ItemName :type Text))
  (bind (_array_element _array_index) (Utilities|Array|ForEachLoopwithBreak (Variables|Default|GetInventoryList))
    (:LoopBody
      (if (Utilities|Enum|Equal(Enum) (Variables|/Game/Overworld/Blueprints/Items/ItemActors/BP_BaseItem.BP_BaseItem_C|GetName (.Item (Utilities|Struct|BreakBP_Inventory _array_element))) ItemName)
        (return (.Item (Utilities|Struct|BreakBP_Inventory _array_element)) _array_index)))))

(fn AddItemtoInventory
  (params (ItemName :type Text))
  (bind (_item _arrayindex) (Inventory|GetItembyName ItemName))
  (Utilities|IsValid _item
    (:Is%20Valid
      (Utilities|Array|SetArrayElem (Variables|Default|GetInventoryList) _arrayindex (Utilities|Struct|MakeBP_Inventory (.Item (Utilities|Struct|BreakBP_Inventory (Utilities|Array|Get(acopy) (Variables|Default|GetInventoryList) _arrayindex))) (+ (.Count (Utilities|Struct|BreakBP_Inventory (Utilities|Array|Get(acopy) (Variables|Default|GetInventoryList) _arrayindex))) 1))))
    (:Is%20Not%20Valid
      (bind _returnvalue (Game|SpawnActorfromClass "/Game/Overworld/Blueprints/Items/ItemActors/BP_BaseItemUsable.BP_BaseItemUsable_C" (Transformation|GetActorTransform) "Undefined" 0 0))
      (Variables|/Game/Overworld/Blueprints/Items/ItemActors/BP_BaseItem.BP_BaseItem_C|SetName _returnvalue ItemName)
      (Utilities|Array|Add (Variables|Default|GetInventoryList) (Utilities|Struct|MakeBP_Inventory _returnvalue 1)))))

(fn RemoveItemfromInventory
  (params (ItemName :type Text))
  (bind _inventorylist (Variables|Default|GetInventoryList))
  (bind (_item _arrayindex) (Inventory|GetItembyName ItemName))
  (Utilities|IsValid _item
    (:Is%20Valid
      (if (> (- (.Count (Utilities|Struct|BreakBP_Inventory (Utilities|Array|Get(acopy) (Variables|Default|GetInventoryList) _arrayindex))) 1) 0)
        (Utilities|Array|Add _inventorylist (Utilities|Struct|MakeBP_Inventory (.Item (Utilities|Struct|BreakBP_Inventory (Utilities|Array|Get(acopy) (Variables|Default|GetInventoryList) _arrayindex))) (- (.Count (Utilities|Struct|BreakBP_Inventory (Utilities|Array|Get(acopy) (Variables|Default|GetInventoryList) _arrayindex))) 1))))
      (Utilities|Array|RemoveIndex _inventorylist _arrayindex))))

(fn GetUsableItembyName
  (params (ItemName :type Text))
  (bind _array_element (Utilities|Array|ForEachLoopwithBreak (Variables|Default|GetInventoryList))
    (:LoopBody
      (if (Utilities|Enum|Equal(Enum) (Variables|/Game/Overworld/Blueprints/Items/ItemActors/BP_BaseItem.BP_BaseItem_C|GetName (.Item (Utilities|Struct|BreakBP_Inventory _array_element))) ItemName)
        (bind _asbp_base_item_usable (Utilities|Casting|CastToBP_BaseItemUsable (.Item (Utilities|Struct|BreakBP_Inventory _array_element))))
        (return _asbp_base_item_usable 0)))))

(fn DrawInventoryWidget
  (Widget|RemovefromParent (Variables|Default|GetInventoryWidget))
  (bind _returnvalue (UserInterface|CreateWidget "/Game/Overworld/Widgets/WT_Inventory.WT_Inventory_C"))
  (Widget|SetKeyboardFocus _returnvalue)
  (bind _output_get (Variables|Default|SetInventoryWidget _returnvalue))
  (Variables|/Game/Overworld/Widgets/WT_Inventory.WT_Inventory_C|SetPlayer _output_get self)
  (UserInterface|Viewport|AddtoViewport _returnvalue 0))

(fn AddExptoAttribute
  (params (Attribute :type Integer) (AttributeName :type Name))
  (bind _expstruct (Attributes|GetAttributeExpStructbyName (Variables|Default|GetAttributes) AttributeName))
  (Attributes|CheckforAttributeLevelUp _expstruct Attribute AttributeName))

(fn CheckforAttributeLevelUp
  (params (Attribute :type S%20Attribute%20Exp%20Structure) (ExperienceToAdd :type Integer) (AttributeName :type Name))
  (bind (_level _actualexp _nextlevelexp) (Utilities|Struct|BreakS_AttributeExp Attribute))
  (bind _returnvalue (+ _actualexp ExperienceToAdd))
  (LocalVariables|SetAttName AttributeName)
  (if (>= _returnvalue _nextlevelexp)
    (bind _result (Math|Integer|IncrementInt _level)
      (:%20%20
        (LocalVariables|SetActualExp (- _returnvalue _nextlevelexp))
        (LocalVariables|SetNewLevel _result)
        (bind _nextlevelexp_2 (Attributes|GetNextLevelExpfromDataTable (LocalVariables|GetNewLevel) (LocalVariables|GetAttName)))
        (LocalVariables|SetNextLevelExp _nextlevelexp_2)))
    (else
      (LocalVariables|SetActualExp _returnvalue)
      (LocalVariables|SetNewLevel _level)
      (LocalVariables|SetNextLevelExp _nextlevelexp)))
  (Attributes|SetExpAttributesbyAttributeName (LocalVariables|GetAttName) (LocalVariables|GetActualExp) (LocalVariables|GetNextLevelExp) (LocalVariables|GetNewLevel)))

(fn GetAttributeExpStructbyName
  (params (Attributes :type S%20Attributes%20Structure) (AttributeName :type Name))
  (bind (_strength _defense _intelligence _faith _dexterity _speed _health) (Utilities|Struct|BreakS_Attributes Attributes))
  (switch name AttributeName
    (:Strength
      (return _strength))
    (:Defence
      (return _defense))
    (:Intelligence
      (return _intelligence))
    (:Faith
      (return _faith))
    (:Dexterity
      (return _dexterity))
    (:Speed
      (return _speed))
    (:Health
      (return _health))))

(fn SetExpAttributesbyAttributeName
  (params (AttributeName :type Name) (ActualExp :type Integer) (NextLevelExp :type Integer) (NewLevel :type Integer))
  (bind _s_attributeexp (Utilities|Struct|MakeS_AttributeExp NewLevel ActualExp NextLevelExp))
  (switch name AttributeName
    (:Strength
      (Utilities|Struct|SetmembersinS_Attributes (Variables|Default|GetAttributes) _s_attributeexp)
      (return))
    (:Defence
      (Utilities|Struct|SetmembersinS_Attributes (Variables|Default|GetAttributes) _s_attributeexp)
      (return))
    (:Intelligence
      (Utilities|Struct|SetmembersinS_Attributes (Variables|Default|GetAttributes) _s_attributeexp)
      (return))
    (:Faith
      (Utilities|Struct|SetmembersinS_Attributes (Variables|Default|GetAttributes) _s_attributeexp)
      (return))
    (:Dexterity
      (Utilities|Struct|SetmembersinS_Attributes (Variables|Default|GetAttributes) _s_attributeexp)
      (return))
    (:Speed
      (Utilities|Struct|SetmembersinS_Attributes (Variables|Default|GetAttributes) _s_attributeexp)
      (return))
    (:Health
      (Utilities|Struct|SetmembersinS_Attributes (Variables|Default|GetAttributes) _s_attributeexp)
      (return))))

(fn GetNextLevelExpfromDataTable
  (params (NewLevel :type Integer) (AttributeName :type Name))
  (bind _returnvalue (Utilities|GetDataTableRow "/Game/Overworld/Blueprints/Player/attributeLevel.attributeLevel" (Utilities|String|StringToName (Utilities|String|ToString(Integer) NewLevel)))
    (:then
      (switch name AttributeName
        (:Strength
          (return (.Strength (Utilities|Struct|BreakS_AttributesNextLevelExp _returnvalue))))
        (:Defence
          (return (.Defense (Utilities|Struct|BreakS_AttributesNextLevelExp _returnvalue))))
        (:Intelligence
          (return (.Intelligence (Utilities|Struct|BreakS_AttributesNextLevelExp _returnvalue))))
        (:Faith
          (return (.Faith (Utilities|Struct|BreakS_AttributesNextLevelExp _returnvalue))))
        (:Dexterity
          (return (.Dexterity (Utilities|Struct|BreakS_AttributesNextLevelExp _returnvalue))))
        (:Speed
          (return (.Speed (Utilities|Struct|BreakS_AttributesNextLevelExp _returnvalue))))
        (:Health
          (return (.Health (Utilities|Struct|BreakS_AttributesNextLevelExp _returnvalue))))))))

(fn SetEquipmentbySlotName
  (params (Item :type BP%20Base%20Item%20Equippable%20Object%20Reference) (SlotName :type E_EquipmentSlots%20Enum :default "NewEnumerator0"))
  (switch Utilities|FlowControl|Switch|SwitchonE_EquipmentSlots SlotName
    (:NewEnumerator0
      (bind _asbp_head_gear (Utilities|Casting|CastToBP_HeadGear Item)
        (:then
          (Utilities|Struct|SetmembersinS_Equipment (Variables|Default|GetEquipment) _asbp_head_gear))
        (:CastFailed
          (Utilities|Struct|SetmembersinS_Equipment (Variables|Default|GetEquipment)))))
    (:NewEnumerator1
      (bind _asbp_chest_gear (Utilities|Casting|CastToBP_ChestGear Item)
        (:then
          (Utilities|Struct|SetmembersinS_Equipment (Variables|Default|GetEquipment) _asbp_chest_gear))
        (:CastFailed
          (Utilities|Struct|SetmembersinS_Equipment (Variables|Default|GetEquipment)))))
    (:NewEnumerator2
      (bind _asbp_leg_gear (Utilities|Casting|CastToBP_LegGear Item)
        (:then
          (Utilities|Struct|SetmembersinS_Equipment (Variables|Default|GetEquipment) _asbp_leg_gear))
        (:CastFailed
          (Utilities|Struct|SetmembersinS_Equipment (Variables|Default|GetEquipment)))))
    (:NewEnumerator3
      (bind _asbp_foot_gear (Utilities|Casting|CastToBP_FootGear Item)
        (:then
          (Utilities|Struct|SetmembersinS_Equipment (Variables|Default|GetEquipment) _asbp_foot_gear))
        (:CastFailed
          (Utilities|Struct|SetmembersinS_Equipment (Variables|Default|GetEquipment)))))
    (:NewEnumerator4
      (bind _asbp_hand_gear (Utilities|Casting|CastToBP_HandGear Item)
        (:then
          (Utilities|Struct|SetmembersinS_Equipment (Variables|Default|GetEquipment) _asbp_hand_gear))
        (:CastFailed
          (Utilities|Struct|SetmembersinS_Equipment (Variables|Default|GetEquipment)))))
    (:NewEnumerator5
      (bind _asbp_base_item_weapon (Utilities|Casting|CastToBP_BaseItemWeapon Item)
        (:then
          (Utilities|Struct|SetmembersinS_Equipment (Variables|Default|GetEquipment) _asbp_base_item_weapon))
        (:CastFailed
          (Utilities|Struct|SetmembersinS_Equipment (Variables|Default|GetEquipment)))))
    (:NewEnumerator6
      (bind _asbp_base_item_weapon_2 (Utilities|Casting|CastToBP_BaseItemWeapon Item)
        (:then
          (Utilities|Struct|SetmembersinS_Equipment (Variables|Default|GetEquipment) _asbp_base_item_weapon_2))
        (:CastFailed
          (Utilities|Struct|SetmembersinS_Equipment (Variables|Default|GetEquipment)))))))