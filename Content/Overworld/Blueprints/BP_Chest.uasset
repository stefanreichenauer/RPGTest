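; BP_Chest is an overworld chest actor that reports the items it contains when opened by a nearby player.
; Begin and end overlap events with BP_OverworldPlayer toggle a PlayerInTrigger flag and print debug messages.
; OpenChest, while that flag is set, looks up each ContainedItems row name in ItemObjectTable and prints the item name.
; It only prints the items and does not grant or remove them.
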(event Custom|OpenChest
  (if (Variables|Default|GetPlayerInTrigger)
    (for _array_element (Variables|Default|GetContainedItems)
      (bind _returnvalue (Utilities|GetDataTableRow "/Game/DataTables/ItemObjectTable.ItemObjectTable" _array_element)
        (:then
          (Development|PrintString (Utilities|String|Append "Item in chest: " (Utilities|String|EnumtoString (.Name (Utilities|Struct|BreakItemObjectAttributes _returnvalue))))))))))

(event EventBeginPlay)

(event Collision|EventActorBeginOverlap
  (params (OtherActor :type Actor%20Object%20Reference))
  (Utilities|Casting|CastToBP_OverworldPlayer OtherActor)
  (Variables|Default|SetPlayerInTrigger true)
  (Development|PrintString "intrigger"))

(event EventTick
  (params (DeltaSeconds :type Float%20%28single-precision%29)))

(event Collision|EventActorEndOverlap
  (params (OtherActor :type Actor%20Object%20Reference))
  (Utilities|Casting|CastToBP_OverworldPlayer OtherActor)
  (Variables|Default|SetPlayerInTrigger false)
  (Development|PrintString "outoftrigger"))

(fn ConstructionScript)