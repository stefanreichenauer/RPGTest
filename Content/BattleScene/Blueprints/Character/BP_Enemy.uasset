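; BP_Enemy is the enemy character for the battle scene, exposing combat stats and taking damage.
; DoDamage subtracts from Health, notifies the BattleMenu through the game instance's BattleScene, and prints a debug health message.
; Defense sums the defence of five equipped gear pieces.
; Attack power and max health are hardcoded, while the mana and equipment getters are unimplemented stubs.
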(event EventBeginPlay)

(event Collision|EventActorBeginOverlap
  (params (OtherActor :type Actor%20Object%20Reference)))

(event EventTick
  (params (DeltaSeconds :type Float%20%28single-precision%29)))

(event EventDoDamage
  (params (Damage :type Integer))
  (Variables|Default|SetHealth (- (Variables|Default|GetHealth) (Math|Conversions|ToFloat(Integer) Damage)))
  (bind _asbp_my_game_instance (Utilities|Casting|CastToBP_MyGameInstance (Game|GetGameInstance)))
  (Default|OnCharacterHealthChanged (Variables|/Game/BattleScene/Blueprints/BP_BattleScene.BP_BattleScene_C|GetBattleMenu (Variables|/Game/GameInstance/BP_MyGameInstance.BP_MyGameInstance_C|GetBattleScene _asbp_my_game_instance)) self "NewEnumerator4")
  (Development|PrintString (Utilities|String|Append "Enemy Health: " (Utilities|String|ToString(Integer) (Math|Float|Truncate (- (Variables|Default|GetHealth) (Math|Conversions|ToFloat(Integer) Damage)))))))

(fn ConstructionScript)

(fn GetActualHealth
  (return (Math|Float|Truncate (Variables|Default|GetHealth))))

(fn GetActualMana)

(fn GetAttackPower
  (return 0))

(fn GetAttributes
  (return (Variables|Default|GetAttributes)))

(fn GetDefense
  (bind _equipment (Variables|Default|GetEquipment))
  (bind (_headgear _chestgear _leggear _footgear _handgear) (Utilities|Struct|BreakS_Equipment _equipment))
  (return (+ (Variables|/Game/Overworld/Blueprints/Items/ItemActors/Equippable/Armor/BP_BaseItemArmor.BP_BaseItemArmor_C|GetDefence _headgear) (Variables|/Game/Overworld/Blueprints/Items/ItemActors/Equippable/Armor/BP_BaseItemArmor.BP_BaseItemArmor_C|GetDefence _chestgear) (Variables|/Game/Overworld/Blueprints/Items/ItemActors/Equippable/Armor/BP_BaseItemArmor.BP_BaseItemArmor_C|GetDefence _leggear) (Variables|/Game/Overworld/Blueprints/Items/ItemActors/Equippable/Armor/BP_BaseItemArmor.BP_BaseItemArmor_C|GetDefence _footgear) (Variables|/Game/Overworld/Blueprints/Items/ItemActors/Equippable/Armor/BP_BaseItemArmor.BP_BaseItemArmor_C|GetDefence _handgear))))

(fn GetEquipment
  (return ""))

(fn GetMaxHealth
  (return 100))

(fn GetMaxMana)