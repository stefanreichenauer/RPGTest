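; Player pawn for the battle scene that opens the battle menu in UI-only input and notifies BattleScene.
; On BeginPlay it also spawns and equips a BP_HeadGear with hardcoded defence.
; Attack power and defense come from game-instance equipment, but Attack subtracts fixed damage from a BP_Enemy's health.
; Health, mana and equipment getters are stubs, and the V key prints the primary weapon name for debugging.
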(event EventBeginPlay
  (bind _returnvalue (UserInterface|CreateWidget "/Game/BattleScene/Widgets/WT_BattleMenu.WT_BattleMenu_C"))
  (UserInterface|Viewport|AddtoViewport _returnvalue 0)
  (bind _output_get (Variables|Default|SetBattleMenu _returnvalue))
  (Input|SetInputModeUIOnly (Game|GetPlayerController 0) _output_get "DoNotLock")
  (Default|OnWidgetSet (Variables|Default|GetBattleScene))
  (bind _returnvalue_2 (Game|SpawnActorfromClass "/Game/Overworld/Blueprints/Items/ItemActors/Equippable/Armor/BP_HeadGear.BP_HeadGear_C" (Transformation|GetActorTransform) "Undefined" 0 0))
  (Variables|/Game/Overworld/Blueprints/Items/ItemActors/Equippable/Armor/BP_BaseItemArmor.BP_BaseItemArmor_C|SetDefence _returnvalue_2 20)
  (Utilities|Struct|SetmembersinS_Equipment (Variables|Default|GetEquipment) _returnvalue_2))

(event Collision|EventActorBeginOverlap
  (params (OtherActor :type Actor%20Object%20Reference)))

(event EventTick
  (params (DeltaSeconds :type Float%20%28single-precision%29)))

(event Input|KeyboardEvents|V
  (params (Key :type Key%20Structure))
  (:Pressed
    (bind _asbp_my_game_instance (Utilities|Casting|CastToBP_MyGameInstance (Game|GetGameInstance)))
    (Development|PrintString "Hello")
    (Development|PrintString (Utilities|String|ToString(Text) (Variables|/Game/Overworld/Blueprints/Items/BP_BaseItemObject.BP_BaseItemObject_C|GetName (Utilities|Struct|BreakS_EquipmentObjects (Variables|/Game/Overworld/Blueprints/Equipment/BP_EquipmentClass.BP_EquipmentClass_C|GetEquipment (Variables|/Game/GameInstance/BP_PlayerCharacteristics.BP_PlayerCharacteristics_C|GetEquipment (Variables|/Game/GameInstance/BP_MyGameInstance.BP_MyGameInstance_C|GetPlayerCharacteristics _asbp_my_game_instance)))))))))

(fn ConstructionScript)

(fn Attack
  (params (Target :type I%20Character%20Interface))
  (bind _asbp_enemy (Utilities|Casting|CastToBP_Enemy Target))
  (Variables|/Game/BattleScene/Blueprints/Character/BP_Enemy.BP_Enemy_C|SetHealth _asbp_enemy (- (Variables|/Game/BattleScene/Blueprints/Character/BP_Enemy.BP_Enemy_C|GetHealth _asbp_enemy) 1e+01)))

(fn GetActualHealth)

(fn GetActualMana)

(fn GetAttackPower
  (bind _asbp_my_game_instance (Utilities|Casting|CastToBP_MyGameInstance (Game|GetGameInstance)))
  (return (Variables|/Game/Overworld/Blueprints/Items/Weapons/BP_WeaponItem.BP_WeaponItem_C|GetPower (Utilities|Struct|BreakS_EquipmentObjects (Variables|/Game/Overworld/Blueprints/Equipment/BP_EquipmentClass.BP_EquipmentClass_C|GetEquipment (Variables|/Game/GameInstance/BP_PlayerCharacteristics.BP_PlayerCharacteristics_C|GetEquipment (Variables|/Game/GameInstance/BP_MyGameInstance.BP_MyGameInstance_C|GetPlayerCharacteristics _asbp_my_game_instance)))))))

(fn GetAttributes
  (return (Variables|Default|GetAttributes)))

(fn GetDefense
  (bind _asbp_my_game_instance (Utilities|Casting|CastToBP_MyGameInstance (Game|GetGameInstance)))
  (return (Variables|/Game/Overworld/Blueprints/Equipment/BP_EquipmentClass.BP_EquipmentClass_C|GetEquipmentDefense (Variables|/Game/GameInstance/BP_PlayerCharacteristics.BP_PlayerCharacteristics_C|GetEquipment (Variables|/Game/GameInstance/BP_MyGameInstance.BP_MyGameInstance_C|GetPlayerCharacteristics _asbp_my_game_instance)))))

(fn GetEquipment
  (return ""))

(fn GetMaxHealth)

(fn GetMaxMana)