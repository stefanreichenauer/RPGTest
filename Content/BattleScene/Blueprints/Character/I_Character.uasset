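; I_Character is a Blueprint interface for characters in the battle scene, declaring their shared combat contract.
; It exposes getters for attributes, defense, attack power, and maximum and current health and mana.
; DoDamage takes a damage input and OnDeath signals death, with all logic left to implementing classes.
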(fn GetAttributes
  (return ""))

(fn GetDefense
  (return 0))

(fn GetAttackPower
  (return 0))

(fn DoDamage
  (params (Damage :type Integer)))

(fn GetMaxHealth
  (return 0))

(fn GetActualHealth
  (return 0))

(fn GetMaxMana
  (return 0))

(fn GetActualMana
  (return 0))

(fn OnDeath)