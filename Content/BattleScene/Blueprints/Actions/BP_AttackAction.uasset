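; Battle action Blueprint that makes a User attack a Target, applying the calculated damage through DoDamage.
; CalculateDamage sums the User's attribute levels weighted by the Attack's influence list, and does the same for the Target with the defense influences.
; Each sum is multiplied by attack power or defense respectively, and their difference, floored at zero, is the damage.
; GetAttributeValue maps each attribute name to its field in the attributes data.
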(event EventDoAction
  (bind _damage (CallFunction|CalculateDamage (Variables|Default|GetAttack)))
  (Default|DoDamage (Variables|Default|GetTarget) _damage))

(fn CalculateDamage
  (params (Attack :type S%20Attacks%20Structure))
  (bind (_name _attackinfluence _defenseinfluences) (Utilities|Struct|BreakS_Attacks Attack))
  (bind _attributes (Default|GetAttributes (Variables|Default|GetUser)))
  (for _array_element _attackinfluence
    (bind _outattribute (CallFunction|GetAttributeValue (.Attribute (Utilities|Struct|BreakS_AttackInfluences _array_element)) _attributes))
    (Variables|Default|SetDamageValue (+ (Variables|Default|GetDamageValue) (* (Utilities|Struct|BreakS_AttributeExp _outattribute) (.Value (Utilities|Struct|BreakS_AttackInfluences _array_element))))))
  (bind _attributes_2 (Default|GetAttributes (Variables|Default|GetTarget)))
  (for _array_element_2 _defenseinfluences
    (bind _outattribute_2 (CallFunction|GetAttributeValue (.attribute _array_element_2) _attributes_2))
    (Variables|Default|SetDefenseValue (+ (Variables|Default|GetDefenseValue) (* (Utilities|Struct|BreakS_AttributeExp _outattribute_2) (.value _array_element_2)))))
  (bind _attackpower (Default|GetAttackPower (Variables|Default|GetUser)))
  (bind _defence (Default|GetDefense (Variables|Default|GetTarget)))
  (if (<= (- (* _attackpower (Variables|Default|GetDamageValue)) (* _defence (Variables|Default|GetDefenseValue))) 0)
    (return 0)
    (else
      (return (- (* _attackpower (Variables|Default|GetDamageValue)) (* _defence (Variables|Default|GetDefenseValue)))))))

(fn GetAttributeValue
  (params (AttributeName :type E_Attributes%20Enum :default "NewEnumerator0") (Attribute :type S%20Attributes%20Structure))
  (bind (_strength _defense _intelligence _faith _dexterity _speed _health) (Utilities|Struct|BreakS_Attributes Attribute))
  (switch Utilities|FlowControl|Switch|SwitchonE_Attributes AttributeName
    (:NewEnumerator0
      (return _strength))
    (:NewEnumerator1
      (return _defense))
    (:NewEnumerator2
      (return _intelligence))
    (:NewEnumerator3
      (return _faith))
    (:NewEnumerator4
      (return _dexterity))
    (:NewEnumerator5
      (return _speed))
    (:NewEnumerator6
      (return _health))))