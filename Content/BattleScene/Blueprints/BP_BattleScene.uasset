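; BP_BattleScene sets up and owns a battle on a separate level, returning to the Overworld level when it ends.
; BeginPlay chains macros that define six fixed waypoints, register the scene in the game instance, spawn an enemy, place the player and create a BP_BattleHandler object.
; Occupied waypoints track their character and join an active list.
; OnWidgetSet links the player's battle menu to the enemy and scene.
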(event Custom|OnWidgetSet
  (bind _output_get (Variables|Default|SetBattleMenu (Variables|/Game/BattleScene/Blueprints/Character/BP_BattlePlayer.BP_BattlePlayer_C|GetBattleMenu (Variables|Default|GetPlayer))))
  (Variables|/Game/BattleScene/Widgets/WT_BattleMenu.WT_BattleMenu_C|SetEnemy _output_get (Variables|Default|GetEnemy))
  (Variables|/Game/BattleScene/Widgets/WT_BattleMenu.WT_BattleMenu_C|SetBattleScene _output_get self)
  (Default|ShowStatusBoxes _output_get))

(event EventBeginPlay
  (Utilities|SetWaypoints
    (:Out
      (Utilities|SetBattleSceneinGameInstance
        (:Out
          (Utilities|SpawnEnemy
            (:Out
              (Utilities|SetPlayer
                (:Out
                  (Utilities|SetBattleHandler
                    (:Out
                      (Utilities|Array|Add (Variables|Default|GetPlayers) (Variables|Default|GetPlayer)))))))))))))

(event Collision|EventActorBeginOverlap
  (params (OtherActor :type Actor%20Object%20Reference)))

(event EventTick
  (params (DeltaSeconds :type Float%20%28single-precision%29)))

(fn ConstructionScript)

(fn GetWaypoint
  (params (Waypoint :type E_Waypoints%20Enum :default "NewEnumerator0"))
  (bind _waypoints (Variables|Default|GetWaypoints))
  (bind (_playerwaypoint _playerhelperwaypoint1 _playerhelperwaypoint2 _enemywaypoint1 _enemywaypoint2 _enemywaypoint3) (Utilities|Struct|BreakS_Battlefield _waypoints))
  (switch Utilities|FlowControl|Switch|SwitchonE_Waypoints Waypoint
    (:NewEnumerator0
      (return _playerwaypoint))
    (:NewEnumerator1
      (return _playerhelperwaypoint1))
    (:NewEnumerator2
      (return _playerhelperwaypoint2))
    (:NewEnumerator3
      (return _enemywaypoint1))
    (:NewEnumerator4
      (return _enemywaypoint2))
    (:NewEnumerator5
      (return _enemywaypoint3))))

(fn EndBattle
  (Game|OpenLevel(byName) "Overworld"))