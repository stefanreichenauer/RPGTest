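; BP_BattleHandler queues a battle turn's actions by speed and executes them.
; AddActionToTurn rebuilds TurnActions with faster actions first, though its unguarded comparison inserts a new action before every entry it matches or outpaces.
; EvaluateTurn fires all actions in one loop, setting a timer on an empty DoAction function.
; The Evaluate graph also loops through them, with a latent three-second delay inside the loop.
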(fn AddActiontoTurn
  (params (Action :type I%20Actions%20Interface) (Speed :type Integer))
  (bind _s_turnaction (Utilities|Struct|MakeS_TurnAction Action Speed))
  (bind _tempturnarray (LocalVariables|GetTempTurnArray))
  (if (> (Utilities|Array|Length (Variables|Default|GetTurnActions)) 0)
    (for _array_element (Variables|Default|GetTurnActions)
      (if (>= Speed (Utilities|Struct|BreakS_TurnAction _array_element))
        (LocalVariables|SetValueSet true)
        (Utilities|Array|Add _tempturnarray _s_turnaction))
      (Utilities|Array|Add _tempturnarray _array_element))
    (if (LocalVariables|GetValueSet)
      _
      (else
        (Utilities|Array|Add (LocalVariables|GetTempTurnArray) _s_turnaction)))
    (Variables|Default|SetTurnActions (LocalVariables|GetTempTurnArray))
    (else
      (Utilities|Array|Add (Variables|Default|GetTurnActions) _s_turnaction))))

(fn EvaluateTurn
  (for _array_element (Variables|Default|GetTurnActions)
    (Default|DoAction (.Action (Utilities|Struct|BreakS_TurnAction _array_element)))
    (Utilities|Time|SetTimerbyFunctionName 0 "DoAction" 3.0)))

(fn DoAction)