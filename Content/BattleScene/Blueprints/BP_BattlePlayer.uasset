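; BP_BattlePlayer is the player in the battle scene, apparently still a prototype with key-driven test actions and stubbed getters for attack power and equipment.
; On BeginPlay it creates the battle menu, notifies BattleScene, and spawns headgear into its local Equipment struct.
; F deals fixed damage to the scene's enemy, while H and V print defense and Strength progression.
; Defense and Strength come from BP_MyGameInstance, so the spawned headgear's defense is not read here.
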(event EventBeginPlay
  (bind _returnvalue (UserInterface|CreateWidget "/Game/BattleScene/Widgets/WT_BattleMenu.WT_BattleMenu_C"))
  (UserInterface|Viewport|AddtoViewport _returnvalue 0)
  (Variables|Default|SetBattleMenu _returnvalue)
  (Default|OnWidgetSet (Variables|Default|GetBattleScene))
  (bind _returnvalue_2 (Game|SpawnActorfromClass "/Game/Overworld/Blueprints/Items/ItemActors/Equippable/Armor/BP_HeadGear.BP_HeadGear_C" (Transformation|GetActorTransform) "Undefined" 0 0))
  (Variables|/Game/Overworld/Blueprints/Items/ItemActors/Equippable/Armor/BP_BaseItemArmor.BP_BaseItemArmor_C|SetDefence _returnvalue_2 20)
  (Utilities|Struct|SetmembersinS_Equipment (Variables|Default|GetEquipment) _returnvalue_2))

(event Collision|EventActorBeginOverlap
  (params (OtherActor :type Actor%20Object%20Reference)))

(event EventTick
  (params (DeltaSeconds :type Float%20%28single-precision%29)))

(event Input|KeyboardEvents|V
  (params (Key :type Key%20Structure))
  (:Pressed
    (bind _asbp_my_game_instance (Utilities|Casting|CastToBP_MyGameInstance (Game|GetGameInstance)))
    (Development|PrintString (Utilities|String|Append "Level: " (Utilities|String|ToString(Integer) (.Level (Utilities|Struct|BreakS_AttributeExp (.Strength (Utilities|Struct|BreakS_Attributes (Variables|/Game/GameInstance/BP_MyGameInstance.BP_MyGameInstance_C|GetInstanceAttributes _asbp_my_game_instance))))))))
    (Development|PrintString (Utilities|String|Append "ActualExp: " (Utilities|String|ToString(Integer) (.ActualExp (Utilities|Struct|BreakS_AttributeExp (.Strength (Utilities|Struct|BreakS_Attributes (Variables|/Game/GameInstance/BP_MyGameInstance.BP_MyGameInstance_C|GetInstanceAttributes _asbp_my_game_instance))))))))
    (Development|PrintString (Utilities|String|Append "NextLvlExp: " (Utilities|String|ToString(Integer) (.NextLevelExp (Utilities|Struct|BreakS_AttributeExp (.Strength (Utilities|Struct|BreakS_Attributes (Variables|/Game/GameInstance/BP_MyGameInstance.BP_MyGameInstance_C|GetInstanceAttributes _asbp_my_game_instance))))))))))

(event Input|KeyboardEvents|H
  (params (Key :type Key%20Structure))
  (:Pressed
    (bind _defence (CallFunction|GetDefense))
    (Development|PrintString (Utilities|String|ToString(Integer) _defence))))

(event Input|KeyboardEvents|F
  (params (Key :type Key%20Structure))
  (:Pressed
    (CallFunction|Attack (Variables|/Game/BattleScene/Blueprints/BP_BattleScene.BP_BattleScene_C|GetEnemy (Variables|Default|GetBattleScene)))))

(fn ConstructionScript)

(fn Attack
  (params (Target :type I%20Character%20Interface))
  (bind _asbp_enemy (Utilities|Casting|CastToBP_Enemy Target))
  (Variables|/Game/BattleScene/Blueprints/BP_Enemy.BP_Enemy_C|SetHealth _asbp_enemy (- (Variables|/Game/BattleScene/Blueprints/BP_Enemy.BP_Enemy_C|GetHealth _asbp_enemy) 1e+01)))

(fn GetAttackPower
  (return 0))

(fn GetAttributes
  (return (Variables|Default|GetAttributes)))

(fn GetDefense
  (bind _asbp_my_game_instance (Utilities|Casting|CastToBP_MyGameInstance (Game|GetGameInstance)))
  (return (Variables|/Game/Overworld/Blueprints/Equipment/BP_EquipmentClass.BP_EquipmentClass_C|GetEquipmentDefense (Variables|/Game/GameInstance/BP_PlayerCharacteristics.BP_PlayerCharacteristics_C|GetEquipment (Variables|/Game/GameInstance/BP_MyGameInstance.BP_MyGameInstance_C|GetPlayerCharacteristics _asbp_my_game_instance)))))

(fn GetEquipment
  (return ""))